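; BP_Alien_PlayerController is a player controller that provides debug hotkeys for the alien game.
; Apostrophe and M call toggles for the debug vision cone and alien idle, whose handling lives outside this graph.
; Enter uses a FlipFlop to toggle game pause.
; L and Ñ step global time dilation down or up within a clamped range and print the new value on screen.
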(event Input|KeyboardEvents|DebugKeyM
  (params (Key :type Key%20Structure :default "None") (ActionValue :type Input%20Action%20Value%20Structure))
  (:Pressed
    (Default|CallToggleDebugAlienIdle)))

(event Input|KeyboardEvents|DebugKeyEnter
  (params (Key :type Key%20Structure :default "None") (ActionValue :type Input%20Action%20Value%20Structure))
  (:Pressed
    (bind _isa (Utilities|FlowControl|FlipFlop)
      (:A
        _)
      (:B
        _))
    (Game|SetGamePaused _isa)))

(event Input|KeyboardEvents|DebugKeyL
  (params (Key :type Key%20Structure :default "None") (ActionValue :type Input%20Action%20Value%20Structure))
  (:Pressed
    (bind _output_get (Variables|Default|SetTimeDilation (Math|Float|Clamp(Float) (- (Variables|Default|GetTimeDilation) 0.25) 0.0 4.0)))
    (Utilities|Time|SetGlobalTimeDilation _output_get)
    (Development|PrintString (Utilities|String|Append "Global Time Dilation:" (Utilities|String|ToString(Float) _output_get) "(-0.25)") true true "(R=1.000000,G=0.612886,B=0.000000,A=1.000000)")))

(event Input|KeyboardEvents|DebugKeyÑ
  (params (Key :type Key%20Structure :default "None") (ActionValue :type Input%20Action%20Value%20Structure))
  (:Pressed
    (bind _output_get (Variables|Default|SetTimeDilation (Math|Float|Clamp(Float) (+ (Variables|Default|GetTimeDilation) 0.25) 0.0 4.0)))
    (Utilities|Time|SetGlobalTimeDilation _output_get)
    (Development|PrintString (Utilities|String|Append "Global Time Dilation:" (Utilities|String|ToString(Float) _output_get) "(+0.25)") true true "(R=1.000000,G=0.202592,B=0.000000,A=1.000000)")))

(event Input|KeyboardEvents|DebugKeyApostrophe
  (params (Key :type Key%20Structure :default "None") (ActionValue :type Input%20Action%20Value%20Structure))
  ;[0.15 0.15 0.15 0.5] Toggle Debug Vision Cone
  (:Pressed
    (Default|CallToggleDebugVisionCone)))

(fn ConstructionScript)